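; BP_ObjectExportTool is a utility actor that exports a static mesh, a camera and the map to files under the project's Saved directory.
; Separate functions build paths from object names and pass them to same-named export calls.
; The mesh is written as both JSON and binary .stm, the camera's component as JSON, and the map as a fixed-name Default.map.
; Events and construction script are empty.
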(fn `ExportCamera`
  (bind _camera (`self.Camera`))
  (`ObjectExporterBPLibrary.ExportCamera` (`CameraActor.CameraComponent` _camera) (`KismetStringLibrary.Concat_StrStr` (`KismetSystemLibrary.GetProjectSavedDirectory`) "Json/" (`KismetSystemLibrary.GetObjectName` _camera) ".json")))

(fn `ExportMap`
  (`ObjectExporterBPLibrary.ExportMap` self (`KismetStringLibrary.Concat_StrStr` (`KismetSystemLibrary.GetProjectSavedDirectory`) "Bin/Map/" "Default" ".map")))

(fn `ExportStaticMesh`
  (bind _returnvalue (`KismetSystemLibrary.GetProjectSavedDirectory`))
  (bind _staticmesh (`self.StaticMesh`))
  (bind _returnvalue_2 (`KismetSystemLibrary.GetObjectName` _staticmesh))
  (`ObjectExporterBPLibrary.ExportStaticMesh` _staticmesh (`KismetStringLibrary.Concat_StrStr` _returnvalue "Json/" _returnvalue_2 ".json"))
  (`ObjectExporterBPLibrary.ExportStaticMesh` _staticmesh (`KismetStringLibrary.Concat_StrStr` _returnvalue "Bin/" _returnvalue_2 ".stm")))

(fn `UserConstructionScript`)